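; Floor actor that runs batches of physics-thrown D38 dice and uploads the rolled results to a web server.
; Touching its cube spawns dice with random positions and impulses, while Tick polls for zero velocity.
; Once settled, each die's highest sphere gives its face number, then the dice are destroyed and the next batch starts.
; After the final batch, VaRest POSTs all results as a JSON string array.
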(event `self.Cube.OnInputTouchBegin`
  (params (FingerIndex :type "ETouchIndex Enum" :default "Touch1") (TouchedComponent :type "PrimitiveComponent Object Reference"))
  (if (< (`self.index`) 6)
    (`self.CreateObjectsAndThrow`)))

(event `self.ReceiveBeginPlay`
  (set `self.iterations` 5))

(event `self.ReceiveTick`
  (params (DeltaSeconds :type "Float (single-precision)"))
  (if (`self.isRolling`)
    (for _array_element (`self.diceArray`)
      (if (`KismetMathLibrary.EqualExactly_VectorVector` (`SceneComponent.GetComponentVelocity` (`/Game/d38_BP.d38` _array_element)))
        (set `self.diceHaveStopped` true)
        (else
          (set `self.diceHaveStopped` false)
          (break))))
    (if (`self.diceHaveStopped`)
      (set `self.isRolling` false)
      (`self.GetHighestFace`))))

(event `CreateObjectsAndThrow`
  (`/Engine/EditorBlueprintResources/StandardMacros.IncrementInt` (`self.index`)
    (:`  `
      (for _ (range 30)
        (bind _returnvalue (`|SpawnActorFromClass` "/Game/d38_BP.d38_BP_C" (`KismetMathLibrary.MakeTransform` (`KismetMathLibrary.MakeVector` (+ (`KismetMathLibrary.RandomFloatInRange` -400.0 400.0) (.x (`SceneComponent.K2_GetComponentLocation` (`self.Cube`)))) (+ (`KismetMathLibrary.RandomFloatInRange` -400.0 400.0) (.y (`SceneComponent.K2_GetComponentLocation` (`self.Cube`)))) (+ (`KismetMathLibrary.RandomFloatInRange` 10.0 140.0) (.z (`SceneComponent.K2_GetComponentLocation` (`self.Cube`))))) (`KismetMathLibrary.Conv_VectorToRotator` (`KismetMathLibrary.MakeVector` (`KismetMathLibrary.RandomFloatInRange` 1.0 5.0) (`KismetMathLibrary.RandomFloatInRange` 1.0 5.0) (`KismetMathLibrary.RandomFloatInRange` 1.0 5.0)))) "AlwaysSpawn" "MultiplyWithRoot" null null))
        (`KismetArrayLibrary.Array_Add` (`self.diceArray`) _returnvalue)
        (`PrimitiveComponent.AddImpulse` (`/Game/d38_BP.d38` _returnvalue) (`KismetMathLibrary.MakeVector` (`KismetMathLibrary.RandomFloatInRange` -600.0 600.0) (`KismetMathLibrary.RandomFloatInRange` -600.0 600.0) (`KismetMathLibrary.RandomFloatInRange` 120.0 300.0)) "None" false)
        (`KismetSystemLibrary.Delay` 0.2)
        (set `self.isRolling` true)
        (set `self.diceHaveStopped` false)))))

(event `SendRequest`
  (bind _json_request (`self.JSON Request`))
  (bind _returnvalue (`VaRestRequestJSON.GetRequestObject` (`self.JSON Request`)))
  (bind _returnvalue_2 (`VaRestSubsystem.ConstructVaRestRequestExt` (subsystem `VaRestSubsystem`) "POST" "json"))
  (bind _output_get (set `self.JSON Request` _returnvalue_2))
  (add `VaRestRequestJSON.OnRequestFail` _output_get (delegate `RequestCompleteCallback`))
  (add `VaRestRequestJSON.OnRequestComplete` _output_get (delegate `RequestCompleteCallback`))
  (`VaRestJsonObject.SetStringArrayField` _returnvalue "stringarray" (`self.outputString`))
  (`VaRestRequestJSON.SetRequestObject` _json_request _returnvalue)
  (`VaRestRequestJSON.ProcessURL` _json_request "https://1b6e-2400-adc1-450-1300-c40e-78eb-9326-ec52.ngrok-free.app/data"))

(event `RequestCompleteCallback`
  (params (Request :type "VaRestRequestJSON Object Reference"))
  (`KismetSystemLibrary.PrintString` (`KismetStringLibrary.Conv_IntToString` (`VaRestRequestJSON.GetResponseCode` Request))))

(event `DeleteObjects`
  (for _array_element (`self.diceArray`)
    (`self.K2_DestroyActor` _array_element))
  (`KismetArrayLibrary.Array_Clear` (`self.diceArray`))
  (if (>= (`self.index`) (`self.iterations`))
    (`KismetSystemLibrary.PrintString` "BatchCompleted")
    (`self.SendRequest`)
    (else
      (`self.CreateObjectsAndThrow`))))

(fn `GetHighestFace`
  (locals (NewLocalVar :type Boolean))
  (for _array_element (`self.diceArray`)
    (set `self.highestZ` 120.0)
    (for (_array_element_2 _array_index) (`/Game/d38_BP.sphereArray` _array_element)
      (bind (_x _y _z) (`KismetMathLibrary.BreakVector3f` (`SceneComponent.K2_GetComponentLocation` _array_element_2)))
      (if (> _z (`self.highestZ`))
        (set `self.highestZ` _z)
        (set `self.highestSphere` _array_element_2)
        (set `self.sphereIndex` _array_index)))
    (bind _result (`/Engine/EditorBlueprintResources/StandardMacros.IncrementInt` (`self.sphereIndex`))
      (:`  `
        (bind _output_get (set `self.sphereIndex` _result))
        (`KismetArrayLibrary.Array_Add` (`self.outputArray`) _output_get)
        (bind _returnvalue (`KismetStringLibrary.Conv_IntToString` _output_get))
        (`KismetArrayLibrary.Array_Add` (`self.outputString`) _returnvalue)
        (`KismetSystemLibrary.PrintString` _returnvalue))))
  (`self.DeleteObjects`))

(fn `UserConstructionScript`)