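; Actor Blueprint d38_BP that fills SphereArray with the integers 1 through 38 when play begins.
; BeginPlay builds the list through a hard-coded chain of individual Add calls rather than a loop.
; Nothing in the file reads the array, and the overlap, Tick and construction script graphs hold no logic.
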(event `self.ReceiveBeginPlay`
  (bind _spherearray (`self.sphereArray`))
  (`KismetArrayLibrary.Array_Add` _spherearray (`self.1`))
  (`KismetArrayLibrary.Array_Add` _spherearray (`self.2`))
  (`KismetArrayLibrary.Array_Add` _spherearray (`self.3`))
  (`KismetArrayLibrary.Array_Add` _spherearray (`self.4`))
  (`KismetArrayLibrary.Array_Add` _spherearray (`self.5`))
  (`KismetArrayLibrary.Array_Add` _spherearray (`self.6`))
  (`KismetArrayLibrary.Array_Add` _spherearray (`self.7`))
  (`KismetArrayLibrary.Array_Add` _spherearray (`self.8`))
  (`KismetArrayLibrary.Array_Add` _spherearray (`self.9`))
  (`KismetArrayLibrary.Array_Add` _spherearray (`self.10`))
  (`KismetArrayLibrary.Array_Add` _spherearray (`self.11`))
  (`KismetArrayLibrary.Array_Add` _spherearray (`self.12`))
  (`KismetArrayLibrary.Array_Add` _spherearray (`self.13`))
  (`KismetArrayLibrary.Array_Add` _spherearray (`self.14`))
  (`KismetArrayLibrary.Array_Add` _spherearray (`self.15`))
  (`KismetArrayLibrary.Array_Add` _spherearray (`self.16`))
  (`KismetArrayLibrary.Array_Add` _spherearray (`self.17`))
  (`KismetArrayLibrary.Array_Add` _spherearray (`self.18`))
  (`KismetArrayLibrary.Array_Add` _spherearray (`self.19`))
  (`KismetArrayLibrary.Array_Add` _spherearray (`self.20`))
  (`KismetArrayLibrary.Array_Add` _spherearray (`self.21`))
  (`KismetArrayLibrary.Array_Add` _spherearray (`self.22`))
  (`KismetArrayLibrary.Array_Add` _spherearray (`self.23`))
  (`KismetArrayLibrary.Array_Add` _spherearray (`self.24`))
  (`KismetArrayLibrary.Array_Add` _spherearray (`self.25`))
  (`KismetArrayLibrary.Array_Add` _spherearray (`self.26`))
  (`KismetArrayLibrary.Array_Add` _spherearray (`self.27`))
  (`KismetArrayLibrary.Array_Add` _spherearray (`self.28`))
  (`KismetArrayLibrary.Array_Add` _spherearray (`self.29`))
  (`KismetArrayLibrary.Array_Add` _spherearray (`self.30`))
  (`KismetArrayLibrary.Array_Add` _spherearray (`self.31`))
  (`KismetArrayLibrary.Array_Add` _spherearray (`self.32`))
  (`KismetArrayLibrary.Array_Add` _spherearray (`self.33`))
  (`KismetArrayLibrary.Array_Add` _spherearray (`self.34`))
  (`KismetArrayLibrary.Array_Add` _spherearray (`self.35`))
  (`KismetArrayLibrary.Array_Add` _spherearray (`self.36`))
  (`KismetArrayLibrary.Array_Add` _spherearray (`self.37`))
  (`KismetArrayLibrary.Array_Add` _spherearray (`self.38`)))

(fn `UserConstructionScript`)